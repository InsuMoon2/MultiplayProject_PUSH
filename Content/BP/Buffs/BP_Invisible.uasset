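; BP_Invisible is a buff that makes its owning BP_PushCharacter invisible for as long as it exists.
; If the owner has a valid controller, a timeline animates the mesh's Alpha parameter with IsAlpha enabled.
; Otherwise it caches the materials, animates Amount, then swaps every slot to an M_Invisible dynamic instance.
; On destruction it resets the parameters or restores the cached materials, depending on the same controller check.
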(event EventBeginPlay
  (bind _asbp_push_character (Utilities|Casting|CastToBP_PushCharacter (Components|GetOwner)))
  (Utilities|IsValid (Pawn|GetController _asbp_push_character)
    (:Is%20Valid
      (Rendering|Material|SetScalarParameterValueonMaterials (Variables|/Script/Engine.Character|GetMesh _asbp_push_character) "IsAlpha" 1.0)
      (bind _새_트랙_0 (Timeline|타임라인_1 PlayFromStart)
        (:Update
          (Rendering|Material|SetScalarParameterValueonMaterials (Variables|/Script/Engine.Character|GetMesh _asbp_push_character) "Alpha" _새_트랙_0))))
    (:Is%20Not%20Valid
      (Rendering|Material|SetScalarParameterValueonMaterials (Variables|/Script/Engine.Character|GetMesh _asbp_push_character) "IsAlpha" 0.0)
      (Variables|Default|SetNewVar_0 (Rendering|Material|GetMaterials (Variables|/Script/Engine.Character|GetMesh _asbp_push_character)))
      (bind _새_트랙_0_2 (Timeline|타임라인_0 PlayFromStart)
        (:Update
          (Rendering|Material|SetScalarParameterValueonMaterials (Variables|/Script/Engine.Character|GetMesh _asbp_push_character) "Amount" _새_트랙_0_2))
        (:Finished
          (bind _returnvalue (Rendering|Material|CreateDynamicMaterialInstance (Variables|/Script/Engine.Character|GetMesh _asbp_push_character) 0 "/Game/Mannequin/Character/Materials/M_Invisible.M_Invisible" "None" :!class /Script/Engine.PrimitiveComponent))
          (for (_ _array_index) (Variables|Default|GetNewVar_0)
            (Rendering|Material|SetMaterial (Variables|/Script/Engine.Character|GetMesh _asbp_push_character) _array_index _returnvalue)))))))

(event EventDestroyed
  (bind _asbp_push_character (Utilities|Casting|CastToBP_PushCharacter (Components|GetOwner)))
  (Utilities|IsValid (Pawn|GetController _asbp_push_character)
    (:Is%20Valid
      (Rendering|Material|SetScalarParameterValueonMaterials (Variables|/Script/Engine.Character|GetMesh _asbp_push_character) "IsAlpha" 0.0)
      (Rendering|Material|SetScalarParameterValueonMaterials (Variables|/Script/Engine.Character|GetMesh _asbp_push_character) "Alpha" 0.0))
    (:Is%20Not%20Valid
      (for (_array_element _array_index) (Variables|Default|GetNewVar_0)
        (Rendering|Material|SetMaterial (Variables|/Script/Engine.Character|GetMesh _asbp_push_character) _array_index _array_element))
      (Rendering|Material|SetScalarParameterValueonMaterials (Variables|/Script/Engine.Character|GetMesh _asbp_push_character) "Amount" 1.0))))

(fn ConstructionScript)