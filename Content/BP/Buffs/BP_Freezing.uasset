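; BP_Freezing is a freeze buff actor that applies an icy visual effect to its owning BP_PushCharacter.
; On BeginPlay, a timeline drives the Emissive scalar parameter on the owner's mesh materials.
; On Destroyed, it resets Emissive to zero and spawns the NS_Ice_ArcticPulse system attached to that mesh.
; The graph holds only these visuals, with no gameplay logic.
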(event EventBeginPlay
  (bind _asbp_push_character (Utilities|Casting|CastToBP_PushCharacter (Components|GetOwner)))
  (bind _새_트랙_0 (Timeline|타임라인_0 PlayFromStart)
    (:Update
      (Rendering|Material|SetScalarParameterValueonMaterials (Variables|/Script/Engine.Character|GetMesh _asbp_push_character) "Emissive" _새_트랙_0))))

(event Collision|EventActorBeginOverlap
  (params (OtherActor :type Actor%20Object%20Reference)))

(event EventTick
  (params (DeltaSeconds :type Float%20%28single-precision%29)))

(event EventDestroyed
  (bind _asbp_push_character (Utilities|Casting|CastToBP_PushCharacter (Components|GetOwner)))
  (Rendering|Material|SetScalarParameterValueonMaterials (Variables|/Script/Engine.Character|GetMesh _asbp_push_character) "Emissive" 0.0)
  (Niagara|SpawnSystemAttached "/Game/Assets/MagicSpells/Ice/FX/NS_Ice_ArcticPulse.NS_Ice_ArcticPulse" (Variables|/Script/Engine.Character|GetMesh _asbp_push_character) "None" "0, 0, 0" "0, 0, 0" "KeepRelativeOffset" false))

(fn ConstructionScript)