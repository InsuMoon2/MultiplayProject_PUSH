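; Lobby game mode that shows connected players as characters on lobby platforms.
; At BeginPlay it caches the BP_LobbyPlayerPlatform actors, ordered by numeric actor tags starting at 0.
; Logins and logouts update the controller list, wait through a polling macro until setup finishes, then sync platforms.
; Syncing spawns unplaced players on the first free platform and clears platforms whose controller is no longer listed.
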(event EventBeginPlay
  (|CallParentFunction)
  (CallFunction|SetUpPlatforms))

(event EventPostLogin
  (params (NewPlayer :type Player%20Controller%20Object%20Reference))
  (|CallParentFunction NewPlayer)
  (Utilities|Array|Add (Variables|Default|GetAllPC) NewPlayer)
  (Utilities|IfPlatformsSetUpIsDone
    (:True
      (CallFunction|UpdatePlayersonPlatforms))))

(event EventOnLogout
  (params (ExitingController :type Controller%20Object%20Reference))
  (|CallParentFunction ExitingController)
  (bind _asplayer_controller (Utilities|Casting|CastToPlayerController ExitingController))
  (Utilities|Array|RemoveItem (Variables|Default|GetAllPC) _asplayer_controller)
  (Utilities|IfPlatformsSetUpIsDone
    (:True
      (CallFunction|UpdatePlayersonPlatforms))))

(fn ConstructionScript)

(fn SetUpPlatforms
  (bind _outactors (Actor|GetAllActorsOfClass "/Game/BP/Objects/BP_LobbyPlayerPlatform.BP_LobbyPlayerPlatform_C"))
  (for _index (range 0 (Utilities|Array|LastIndex _outactors))
    (bind _outactors_2 (Actor|GetAllActorsOfClasswithTag "/Game/BP/Objects/BP_LobbyPlayerPlatform.BP_LobbyPlayerPlatform_C" (Utilities|String|StringToName (Utilities|String|ToString(Integer) _index))))
    (Utilities|Array|Add (Variables|Default|GetLobbyPlatforms) (Utilities|Array|Get(acopy) _outactors_2)))
  (Variables|Default|SetbPlatformSetUpDone true))

(fn UpdatePlayersonPlatforms
  (for _array_element (Variables|Default|GetAllPC)
    (LocalVariables|SetLoop_PCAllReadyAdded false)
    (bind _array_element_2 (Utilities|Array|ForEachLoopwithBreak (Variables|Default|GetLobbyPlatforms) :!label _label)
      (:LoopBody
        (if (== (Variables|/Script/Push.LobbyPlayerPlatform|GetPlayerController _array_element_2) _array_element)
          (LocalVariables|SetLoop_PCAllReadyAdded true)
          (goto _label Break)))
      (:Completed
        (if (not (LocalVariables|GetLoop_PCAllReadyAdded))
          (bind _array_element_3 (Utilities|Array|ForEachLoopwithBreak (Variables|Default|GetLobbyPlatforms) :!label _label_2)
            (:LoopBody
              (Utilities|IsValid (Variables|/Script/Push.LobbyPlayerPlatform|GetPlayerController _array_element_3)
                (:Is%20Not%20Valid
                  (Default|SpawnCharacter _array_element_3 _array_element)
                  (goto _label_2 Break)))))))))
  (for _array_element_4 (Variables|Default|GetLobbyPlatforms)
    (if (not (Utilities|Array|ContainsItem (Variables|Default|GetAllPC) (Variables|/Script/Push.LobbyPlayerPlatform|GetPlayerController _array_element_4)))
      (Class|LobbyPlayerPlatform|Clear _array_element_4))))