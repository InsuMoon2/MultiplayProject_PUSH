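; BP_Skill_Boom_P is a skill actor that searches outward for a character to target.
; On BeginPlay a timeline grows the DetectTarget sphere from zero to its maximum radius, updating overlaps as it expands.
; The first overlapping PushCharacter other than the owner is stored as Target, so the expanding sphere favors the nearest one.
; The graph only acquires the target and applies no effect to it.
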(event OnComponentBeginOverlap(DetectTarget)
  (params (OverlappedComponent :type Primitive%20Component%20Object%20Reference) (OtherActor :type Actor%20Object%20Reference) (OtherComp :type Primitive%20Component%20Object%20Reference) (OtherBodyIndex :type Integer) (bFromSweep :type Boolean) (SweepResult :type Hit%20Result%20Structure%20%28by%20ref%29))
  (bind _aspush_character (Utilities|Casting|CastToPushCharacter OtherActor))
  (if (and (!= _aspush_character (Components|GetOwner)) (== (Variables|Default|GetTarget) 0))
    (Variables|Default|SetTarget _aspush_character)))

(event EventBeginPlay
  (bind _새_트랙_0 (Timeline|타임라인_0 PlayFromStart)
    (:Update
      (Components|Sphere|SetSphereRadius (Variables|Default|GetDetectTarget) (Math|Float|Lerp 0.0 1.5e+03 _새_트랙_0) true))))

(fn ConstructionScript)