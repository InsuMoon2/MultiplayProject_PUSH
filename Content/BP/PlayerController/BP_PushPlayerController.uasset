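; Player controller for the Push game mode that starts player list setup and routes chat input.
; On BeginPlay it waits briefly before calling UpdatePlayerList on the game mode, a timing workaround for player data not arriving correctly.
; Enter and mouse wheel keys forward to the chat component.
; A Server-to-multicast debug chain adjusts gold and kills through the resource component, but its entry call is not wired to run.
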(event Custom|Increase%20Gold_Server
  ;[1 1 1] 디버깅
  (CallFunction|IncreaseGoldNMC))

(event Custom|Increase%20Gold_NMC
  ;[1 1 1] 디버깅
  (bind _resourcecomponent (Variables|Default|GetresourceComponent)
    (:then
      (Utilities|FlowControl|Sequence
        (:then_0
          (Class|ResourceComponent|AdjustGoldServer _resourcecomponent 1))
        (:then_1
          (Class|ResourceComponent|AdjustKillServer _resourcecomponent 2))))
    (:else)))

(event EventBeginPlay
  (bind _pushgamemode (Variables|Default|GetPushGameMode))
  ;[1 1 1] 초기 플레이어 데이터 세팅, 딜레이를 안주면 제대로 들어오지 않음. 해결방법을 몰?루겠어서 딜레이로 처리
  (|CallParentFunction)
  (Utilities|FlowControl|Delay 0.2)
  (Utilities|IsValid _pushgamemode
    (:Is%20Valid
      (Class|PushGameMode|UpdatePlayerList _pushgamemode))))

(event Input|KeyboardEvents|F
  (params (Key :type Key%20Structure :default "None"))
  ;[1 1 1] 디버깅
)

(event Input|KeyboardEvents|Enter
  (params (Key :type Key%20Structure :default "None"))
  (:Pressed
    (Default|InputEnter (Variables|Default|GetBP_ChatComponent1))))

(event Input|MouseEvents|MouseWheelUp
  (params (Key :type Key%20Structure :default "None"))
  (:Pressed
    (Default|InputMouseUp (Variables|Default|GetBP_ChatComponent1))))

(event Input|MouseEvents|MouseWheelDown
  (params (Key :type Key%20Structure :default "None"))
  (:Pressed
    (Default|InputMouseDown (Variables|Default|GetBP_ChatComponent1))))

(fn ConstructionScript)