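; BP_LobbyPlayerPlatform is a lobby platform that displays a character for an assigned player.
; SpawnCharacter stores the given player controller, destroys any existing character and spawns a BP_PushCharacter just above the PlayerSpawnTransform component, ignoring collisions.
; The spawned character is only tracked as CurrentCharacter; the graph does not possess it.
; Clear drops the controller reference and destroys that character to empty the platform.
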(event EventSpawnCharacter
  (params (InPlayerController :type Player%20Controller%20Object%20Reference))
  (bind _playerspawntransform (Variables|Default|GetPlayerSpawnTransform))
  (bind _returnvalue (Transformation|GetWorldTransform _playerspawntransform))
  (Variables|Default|SetPlayerController InPlayerController)
  (Utilities|IsValid (Variables|Default|GetCurrentCharacter)
    (:Is%20Valid
      (Actor|DestroyActor (Variables|Default|GetCurrentCharacter)))
    (:Is%20Not%20Valid
      _))
  (bind _returnvalue_2 (Game|SpawnActorfromClass "/Game/BP/Character/BP_PushCharacter.BP_PushCharacter_C" (Math|Transform|MakeTransform (Math|Vector|MakeVector (+ (.x (.location _returnvalue)) 1.0) (+ (.y (.location _returnvalue)) 1.0) (+ (.z (.location _returnvalue)) 84.0)) (.rotation _returnvalue) (.scale _returnvalue)) "AlwaysSpawn" 0 0))
  (Variables|Default|SetCurrentCharacter _returnvalue_2))

(event EventClear
  (Variables|Default|SetPlayerController 0)
  (Utilities|IsValid (Variables|Default|GetCurrentCharacter)
    (:Is%20Valid
      (Actor|DestroyActor (Variables|Default|GetCurrentCharacter))
      (Variables|Default|SetCurrentCharacter 0))))

(fn ConstructionScript)