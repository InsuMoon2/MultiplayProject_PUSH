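; Player character Blueprint that shows the mouse cursor and a crosshair widget on begin play and binds shop, skill and item input.
; B opens the store through ShopComponent, whose slot widgets handle the four Skill actions and the Q/E item keys.
; Hard-coded J and K keys play the Dead montage and spawn a fireball skill actor ahead of the character.
; A water-hit emitter spawn is left unwired.
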(event EventBeginPlay
  (bind _returnvalue (Game|GetPlayerController 0))
  (|CallParentFunction)
  (Variables|/Script/Engine.PlayerController|SetbShowMouseCursor _returnvalue true)
  (bind _returnvalue_2 (UserInterface|CreateWidget "/Game/BP/Widgets/WDG_CrossHair.WDG_CrossHair_C" _returnvalue))
  (UserInterface|Viewport|AddtoViewport _returnvalue_2 0))

(event Input|KeyboardEvents|B
  (params (Key :type Key%20Structure :default "None"))
  (:Pressed
    (Class|ShopComponent|OpenStoreUI (Variables|Default|GetShopComponent))))

(event Input|KeyboardEvents|J
  (params (Key :type Key%20Structure :default "None"))
  (:Pressed
    (Animation|PlayAnimMontage "/Game/Assets/Animations/Montages/Dead.Dead" 1.0 "None")))

(event Input|KeyboardEvents|K
  (params (Key :type Key%20Structure :default "None"))
  (bind _returnvalue (Transformation|GetActorForwardVector))
  (:Pressed
    (Game|SpawnActorfromClass "/Game/MH/BP_Skill_Fireball_P.BP_Skill_Fireball_P_C" (Math|Transform|MakeTransform (+ (Transformation|GetActorLocation) (* _returnvalue 5e+02)) (Math|Conversions|RotationFromXVector _returnvalue) "1,1,1") "Undefined" self 0)))

(event Input|ActionEvents|InputActionSkill1
  (params (Key :type Key%20Structure))
  (:Pressed
    (bind _aswdg_skill_slots (Utilities|Casting|CastToWDG_SkillSlots (Variables|/Script/Push.ShopComponent|GetSkillSlots (Variables|Default|GetShopComponent))))
    (Default|UseSkill _aswdg_skill_slots)))

(event Input|ActionEvents|InputActionSkill2
  (params (Key :type Key%20Structure))
  (:Pressed
    (bind _aswdg_skill_slots (Utilities|Casting|CastToWDG_SkillSlots (Variables|/Script/Push.ShopComponent|GetSkillSlots (Variables|Default|GetShopComponent))))
    (Default|UseSkill _aswdg_skill_slots 1)))

(event Input|ActionEvents|InputActionSkill3
  (params (Key :type Key%20Structure))
  (:Pressed
    (bind _aswdg_skill_slots (Utilities|Casting|CastToWDG_SkillSlots (Variables|/Script/Push.ShopComponent|GetSkillSlots (Variables|Default|GetShopComponent))))
    (Default|UseSkill _aswdg_skill_slots 2)))

(event Input|ActionEvents|InputActionSkill4
  (params (Key :type Key%20Structure))
  (:Pressed
    (bind _aswdg_skill_slots (Utilities|Casting|CastToWDG_SkillSlots (Variables|/Script/Push.ShopComponent|GetSkillSlots (Variables|Default|GetShopComponent))))
    (Default|UseSkill _aswdg_skill_slots 3)))

(event Input|KeyboardEvents|Q
  (params (Key :type Key%20Structure))
  (:Pressed
    (bind _aswdg_item_slots (Utilities|Casting|CastToWDG_ItemSlots (Variables|/Script/Push.ShopComponent|GetItemSlots (Variables|Default|GetShopComponent))))
    (Default|UseItem _aswdg_item_slots)))

(event Input|KeyboardEvents|E
  (params (Key :type Key%20Structure))
  (:Pressed
    (bind _aswdg_item_slots (Utilities|Casting|CastToWDG_ItemSlots (Variables|/Script/Push.ShopComponent|GetItemSlots (Variables|Default|GetShopComponent))))
    (Default|UseItem _aswdg_item_slots 1)))

(fn ConstructionScript
  (|CallParentFunction))